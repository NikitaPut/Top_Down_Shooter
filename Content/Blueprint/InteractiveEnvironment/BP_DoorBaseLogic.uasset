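; Base logic for a sliding door that raises and lowers its mesh when a BP_Character enters separate open and close trigger volumes.
; Two eased MoveComponentTo nodes handle the directions, lifting to MaxDoorHeight or returning to the default relative location, and each trigger stops the opposite move before starting its own.
; IsDoorOpened gates both triggers and flips when a move completes.
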(event OnComponentBeginOverlap(OpenTrigger)
  (params (OverlappedComponent :type Primitive%20Component%20Object%20Reference) (OtherActor :type Actor%20Object%20Reference) (OtherComp :type Primitive%20Component%20Object%20Reference) (OtherBodyIndex :type Integer) (bFromSweep :type Boolean) (SweepResult :type Hit%20Result%20Structure%20%28by%20ref%29))
  (bind _doormesh (Variables|Default|GetDoorMesh))
  (bind _doormesh_2 (Variables|Default|GetDoorMesh))
  (bind _returnvalue (Transformation|GetRelativeTransform _doormesh))
  (Utilities|Casting|CastToBP_Character OtherActor)
  (if (not (Variables|Default|GetIsDoorOpened))
    (Utilities|FlowControl|Sequence
      (:then_0
        (Components|MoveComponentTo _doormesh_2 (Math|Vector|MakeVector 0.0 0.0 0.0) (.rotation (Transformation|GetRelativeTransform _doormesh_2)) true true 0.5 false) ; enters at Stop
      )
      (:then_1
        (Components|MoveComponentTo _doormesh (Math|Vector|MakeVector (.x (.location _returnvalue)) (.y (.location _returnvalue)) (Variables|Default|GetMaxDoorHeight)) (.rotation _returnvalue) true true 0.5 false)
        (Variables|Default|SetIsDoorOpened (not (Variables|Default|GetIsDoorOpened)))))))

(event OnComponentBeginOverlap(CloseTrigger)
  (params (OverlappedComponent :type Primitive%20Component%20Object%20Reference) (OtherActor :type Actor%20Object%20Reference) (OtherComp :type Primitive%20Component%20Object%20Reference) (OtherBodyIndex :type Integer) (bFromSweep :type Boolean) (SweepResult :type Hit%20Result%20Structure%20%28by%20ref%29))
  (bind _doormesh (Variables|Default|GetDoorMesh))
  (bind _doormesh_2 (Variables|Default|GetDoorMesh))
  (bind _returnvalue (Transformation|GetRelativeTransform _doormesh))
  (Utilities|Casting|CastToBP_Character OtherActor)
  (if (Variables|Default|GetIsDoorOpened)
    (Utilities|FlowControl|Sequence
      (:then_0
        (Components|MoveComponentTo _doormesh (Math|Vector|MakeVector (.x (.location _returnvalue)) (.y (.location _returnvalue)) (Variables|Default|GetMaxDoorHeight)) (.rotation _returnvalue) true true 0.5 false) ; enters at Stop
      )
      (:then_1
        (Components|MoveComponentTo _doormesh_2 (Math|Vector|MakeVector 0.0 0.0 0.0) (.rotation (Transformation|GetRelativeTransform _doormesh_2)) true true 0.5 false)
        (Variables|Default|SetIsDoorOpened (not (Variables|Default|GetIsDoorOpened)))))))

(event EventBeginPlay)

(event EventTick
  (params (DeltaSeconds :type Float%20%28single-precision%29)))

(fn ConstructionScript)