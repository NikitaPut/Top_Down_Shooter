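; Top-down player character Blueprint handling camera boom zoom, movement-state input and debug test keys.
; Zoom either steps instantly or glides via a looping timer that consumes a signed leftover distance, clamped to height limits.
; Sprint, walk and aim flags feed ChangeMovementState, with Tick cancelling sprint when velocity strays from the facing direction.
; Debug keys trigger camera shake and fire or death montages, while on-screen prints show movement and weapon state.
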(event EventTick
  (params (DeltaSeconds :type Float%20%28single-precision%29))
  (Utilities|FlowControl|Sequence
    (:then_0
      (if (Variables|Default|GetbSprintEnabled)
        (bind _isallowedtosprint (CallFunction|IsAllowedtoSprint))
        (if (not _isallowedtosprint)
          (Variables|Default|SetbSprintEnabled _isallowedtosprint)
          (Class|SkillBoxUE2TDSCharacter|ChangeMovementState))))
    (:then_1
      (Development|PrintString (Utilities|String|EnumtoString (Variables|Default|GetMovementState)) true false "(R=0.000000,G=0.660000,B=1.000000,A=1.000000)" 0.0))
    (:then_2
      (bind _returnvalue (Class|SkillBoxUE2TDSCharacter|GetCurrentWeapon))
      (Utilities|IsValid _returnvalue
        (:Is%20Valid
          (bind _returnvalue_2 (Class|WeaponDefault|GetWeaponRounds _returnvalue))
          (Development|PrintString (Utilities|String|Append "IsFiring = " (Utilities|String|ToString(Boolean) (Variables|/Script/SkillBox_UE2_TDS.WeaponDefault|GetbWeaponFiring _returnvalue)) "||| IsReloading = " (Utilities|String|ToString(Boolean) (Variables|/Script/SkillBox_UE2_TDS.WeaponDefault|GetbWeaponReloading _returnvalue)) "||| CurrentRounds = " (Utilities|String|ToString(Integer) _returnvalue_2)) true true "(R=0.000000,G=0.068355,B=1.000000,A=1.000000)" 0.0))))))

(event Input|ActionEvents|InputActionSprint
  (params (Key :type Key%20Structure :default "None"))
  (:Pressed
    (bind _isallowedtosprint (CallFunction|IsAllowedtoSprint))
    (if _isallowedtosprint
      (Variables|Default|SetbSprintEnabled true)
      (else
        (Variables|Default|SetbSprintEnabled false :!label _label)))
    (Class|SkillBoxUE2TDSCharacter|ChangeMovementState))
  (:Released
    (goto _label)))

(event Input|ActionEvents|InputActionWalk
  (params (Key :type Key%20Structure :default "None"))
  (:Pressed
    (Variables|Default|SetbWalkEnabled true)
    (Class|SkillBoxUE2TDSCharacter|ChangeMovementState :!label _label))
  (:Released
    (Variables|Default|SetbWalkEnabled false)
    (goto _label)))

(event Input|ActionEvents|InputActionAim
  (params (Key :type Key%20Structure :default "None"))
  (:Pressed
    (Variables|Default|SetbAimEnabled true)
    (Class|SkillBoxUE2TDSCharacter|ChangeMovementState :!label _label))
  (:Released
    (Variables|Default|SetbAimEnabled false)
    (goto _label)))

(event Input|AxisEvents|InputAxisCameraZoom
  (params (AxisValue :type Float%20%28single-precision%29))
  (if (!= AxisValue 0.0)
    (if (Variables|Camera|General|GetSmoothSlide)
      ;[1 1 1] Smooth Zoom
      (if (not (!= (Variables|Camera|Smooth|GetLeftoverCameraMovement) 0.0))
        (Variables|Camera|Smooth|SetLeftoverCameraMovement (* (Variables|Camera|General|GetHeightChangeDelta) (Math|Float|Sign(Float) AxisValue))) ; We use it for two purposes:\n1. As a flag for "whether we are currently in a smooth zoom"\n2. As a cached value for the direction of zoom\n(negative is shortening the distance from camera)
        (bind _returnvalue (Utilities|Time|SetTimerbyFunctionName 0 "SlideCameraSmoothly" (Variables|Camera|Smooth|GetSmoothZoomTick) true))
        (Variables|Camera|Smooth|SetSmoothSlideTimer _returnvalue))
      (else
        (CallFunction|SlideCamera (Math|Float|Clamp(Float) AxisValue -1.0))))))

(event Input|KeyboardEvents|F
  (params (Key :type Key%20Structure :default "None"))
  (:Released
    (CallFunction|ShakeCamera)))

(event Input|KeyboardEvents|SpaceBar
  (params (Key :type Key%20Structure :default "None"))
  (:Pressed
    (if (Variables|Default|GetbAimEnabled)
      (Animation|PlayAnimMontage "/Game/Blueprint/Character/Mannequin/Animations/NewAnimations/NewFire_Rifle_Ironsights_Montage.NewFire_Rifle_Ironsights_Montage" 1.0 "None")
      (else
        (Animation|PlayAnimMontage "/Game/Blueprint/Character/Mannequin/Animations/NewAnimations/NewFire_Rifle_Hip_Montage.NewFire_Rifle_Hip_Montage" 1.0 "None")))))

(event Input|KeyboardEvents|V
  (params (Key :type Key%20Structure :default "None"))
  (:Pressed
    (Animation|Montage|PlayMontage (Variables|Character|GetMesh) "/Game/Blueprint/Character/Mannequin/Animations/NewAnimations/NewDeath_1_Montage.NewDeath_1_Montage")))

(fn ConstructionScript
  (bind _cameraboom (Variables|Default|GetCameraBoom))
  (Variables|/Script/Engine.SpringArmComponent|SetTargetArmLength _cameraboom (Math|Float|Clamp(Float) (Variables|Camera|General|GetHeight) (Variables|Camera|General|GetMinCameraHeight) (Variables|Camera|General|GetMaxCameraHeight)))
  (Transformation|SetRelativeRotation _cameraboom (Variables|Camera|General|GetCameraRotation) false false)
  (Variables|/Script/Engine.SpringArmComponent|SetbEnableCameraLag _cameraboom (Variables|Camera|General|GetFlow))
  (Variables|/Script/Engine.SpringArmComponent|SetCameraLagSpeed _cameraboom (Variables|Camera|General|GetLagSpeed)))

(fn ShakeCamera
  (Camera|PlayWorldCameraShake "/Game/Blueprint/Game/BP_CameraShake.BP_CameraShake_C" (Transformation|GetWorldLocation (Variables|Default|GetTopDownCameraComponent)) 0.0 3e+01))

(fn SlideCamera
  (params (Value :type Float%20%28single-precision%29))
  (Variables|/Script/Engine.SpringArmComponent|SetTargetArmLength (Variables|Default|GetCameraBoom) (Math|Float|Clamp(Float) (+ (Variables|/Script/Engine.SpringArmComponent|GetTargetArmLength (Variables|Default|GetCameraBoom)) (* Value (Variables|Camera|General|GetHeightChangeDelta))) (Variables|Camera|General|GetMinCameraHeight) (Variables|Camera|General|GetMaxCameraHeight))))

(fn SlideCameraSmoothly
  (bind _smoothzoomseconds (Variables|Camera|Smooth|GetSmoothZoomSeconds))
  (bind _smoothzoomtick (Variables|Camera|Smooth|GetSmoothZoomTick))
  (bind _heightchangedelta (Variables|Camera|General|GetHeightChangeDelta))
  (bind _returnvalue (* _heightchangedelta _smoothzoomtick))
  (bind _returnvalue_2 (/ _returnvalue _smoothzoomseconds))
  ;[1 1 1] If we don't have any movement left over to perform, stop the timer
  (if (Math|Float|NearlyEqual(Float) (Variables|Camera|Smooth|GetLeftoverCameraMovement) 0.0 1e-06)
    (Utilities|Time|ClearandInvalidateTimerbyHandle (Variables|Camera|Smooth|GetSmoothSlideTimer))
    (else
      (Variables|Camera|Smooth|SetLeftoverCameraMovement (+ (Variables|Camera|Smooth|GetLeftoverCameraMovement) (* (* (Math|Float|Sign(Float) (Variables|Camera|Smooth|GetLeftoverCameraMovement)) -1.0) _returnvalue_2)))
      ;[1 1 1] Increment/Decrement Target Arm Length
      (Variables|/Script/Engine.SpringArmComponent|SetTargetArmLength (Variables|Default|GetCameraBoom) (Math|Float|Clamp(Float) (+ (* (Math|Float|Sign(Float) (Variables|Camera|Smooth|GetLeftoverCameraMovement)) _returnvalue_2) (Variables|/Script/Engine.SpringArmComponent|GetTargetArmLength (Variables|Default|GetCameraBoom))) (Variables|Camera|General|GetMinCameraHeight) (Variables|Camera|General|GetMaxCameraHeight))))))

(fn IsAllowedtoSprint
  (bind _returnvalue (Transformation|GetActorForwardVector))
  (bind _returnvalue_2 (Transformation|GetVelocity))
  (bind _returnvalue_3 (Math|Vector|Normalize _returnvalue_2))
  (bind _returnvalue_4 (Math|Conversions|ToVector2D(Vector) _returnvalue))
  (bind _returnvalue_5 (Math|Conversions|ToVector2D(Vector) _returnvalue_3))
  (bind _returnvalue_6 (Math|Vector2D|DotProduct(2D) _returnvalue_4 _returnvalue_5))
  (bind _returnvalue_7 (Math|Trig|Acos(Degrees) _returnvalue_6))
  (Development|PrintString (Utilities|String|ToString(Vector) _returnvalue) true true "(R=0.000000,G=0.375000,B=0.066258,A=1.000000)" 1.0)
  (Development|PrintString (Utilities|String|ToString(Vector) _returnvalue_3) true true "(R=1.000000,G=0.149158,B=0.000000,A=1.000000)" 1.0)
  (Development|PrintString (Utilities|String|ToString(Float) _returnvalue_7) true true "(R=0.000000,G=0.660000,B=1.000000,A=1.000000)" 1.0)
  (return (< _returnvalue_7 0.2)))